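; BP_Laser is a puzzle laser beam that takes its color from a dynamic material and stretches its mesh to whatever blocks it.
; Each tick a short-offset box trace along its up vector sets beam length, capped at its range.
; Hit changes and sustained hits are reported to actors through BPI_Lasers as LaserBounceMessage.
; CancelTargetHit releases or deactivates the last target and destroys the beam unless overridden, while UpdateID builds appended laser IDs.
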(event `self.ReceiveBeginPlay`
  (`self.Change Color`))

(event `self.ReceiveTick`
  (params (DeltaSeconds :type "Float (single-precision)"))
  (`self.Set End Point`))

(fn `Cancel Target Hit`
  (params (Override :type Boolean))
  (returns (`Remove From Array` :type Boolean))
  (`|ExecutionSequence`
    (:`then_0`
      (bind _lasthitactor (`self.LastHitActor`)
        (:`then`
          (bind _asbp_lasers_parent (cast `/Game/Puzzle3/Lasers/BP_LasersParent` _lasthitactor))
          (if (and (`KismetSystemLibrary.DoesImplementInterface` _asbp_lasers_parent "/Game/Puzzle3/Lasers/BPI_Lasers.BPI_Lasers_C") (`KismetArrayLibrary.Array_IsEmpty` (`/Game/Puzzle3/Lasers/BP_LasersParent.LasersAttached` _asbp_lasers_parent)))
            (message `/Game/Puzzle3/Lasers/BPI_Lasers.LaserBounce` (`self.LastHitActor`) self false (struct))
            (else
              (set `/Game/Puzzle3/Lasers/BP_LasersParent.Active` false _asbp_lasers_parent))))
        (:`else`)))
    (:`then_1`
      (if (`local.Override`)
        (return false)
        (else
          (`self.K2_DestroyActor`)
          (return true))))))

(fn `Change Color`
  (bind _returnvalue (`PrimitiveComponent.CreateDynamicMaterialInstance` (`self.SM_Parent`) 0 "/Game/Puzzle3/Lasers/M_Laser.M_Laser" "None"))
  (`MaterialInstanceDynamic.SetVectorParameterValue` _returnvalue "Color" (`self.LaserColor`)))

(fn `Set End Point`
  (locals (`L-Range` :type "Float (double-precision)" :default 6000.0) (`L-HitInfo` :type "HitResult Structure") (`L-HitActor` :type "Actor Object Reference"))
  (bind _returnvalue (`self.GetActorUpVector`))
  (bind _returnvalue_2 (+ (`self.K2_GetActorLocation`) (* _returnvalue 2.0)))
  (bind _outhit (`KismetSystemLibrary.BoxTraceSingle` _returnvalue_2 (+ _returnvalue_2 (* _returnvalue (`local.L-Range`))) (0.5 0.5 0.5) (struct) "TraceTypeQuery1"))
  (bind _output_get (set `local.L-HitInfo` _outhit))
  (bind (_bblockinghit _binitialoverlap _time _distance _location _impactpoint _normal _impactnormal _physmat _hitactor) (`GameplayStatics.BreakHitResult` _output_get))
  (set `local.L-HitActor` _hitactor)
  (`SceneComponent.SetWorldScale3D` (`self.SM_Parent`) (`KismetMathLibrary.MakeVector` 0.05 0.05 (`KismetMathLibrary.SelectFloat` (/ (+ _distance 1.0) 100.0) (/ (`local.L-Range`) 100.0) _bblockinghit)))
  (`|ExecutionSequence`
    (:`then_0`
      (if (!= (`self.LastHitActor`) (`local.L-HitActor`))
        (if (`KismetSystemLibrary.DoesImplementInterface` (`self.LastHitActor`) "/Game/Puzzle3/Lasers/BPI_Lasers.BPI_Lasers_C")
          (message `/Game/Puzzle3/Lasers/BPI_Lasers.LaserBounce` (`self.LastHitActor`) self false (`local.L-HitInfo`)))
        (elif (`KismetSystemLibrary.DoesImplementInterface` (`local.L-HitActor`) "/Game/Puzzle3/Lasers/BPI_Lasers.BPI_Lasers_C")
          (message `/Game/Puzzle3/Lasers/BPI_Lasers.LaserBounce` (`local.L-HitActor`) self true (`local.L-HitInfo`)))))
    (:`then_1`
      (bind _l_hitactor (`local.L-HitActor`)
        (:`then`
          (set `self.LastHitActor` _l_hitactor))
        (:`else`)))))

(fn `Update ID`
  (params (`P-Append` :type String))
  (returns (ReturnValue :type String))
  (return (`KismetStringLibrary.Concat_StrStr` (`self.Laser_ID`) `P-Append`)))

(fn `UserConstructionScript`
  (`parent.UserConstructionScript`))