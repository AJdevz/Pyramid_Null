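; BP_LaserTarget is a laser puzzle target that changes color in response to laser hits.
; LaserBounce stores the hit response as its Active flag and passes the incoming laser's color to PuzzleSolved.
; PuzzleSolved creates a dynamic M_TargetHit material on SMParent, setting Base Color to the laser color when active or a fixed red when inactive.
; It only updates this visual; no further puzzle logic runs here.
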(fn `LaserBounce`
  (params (`P-LaserHit` :type "/Game/Puzzle3/Lasers/BP_Laser Object Reference") (`P-HitResponse` :type Boolean) (`P-HitInformation` :type "HitResult Structure"))
  (returns (`New Laser` :type "/Game/Puzzle3/Lasers/BP_Laser Object Reference"))
  (set `self.Active` `P-HitResponse`)
  (`self.Puzzle Solved` (`/Game/Puzzle3/Lasers/BP_LasersParent.LaserColor` `P-LaserHit`))
  (return null))

(fn `Puzzle Solved`
  (params (`Color Laser` :type "LinearColor Structure"))
  (bind _returnvalue (`PrimitiveComponent.CreateDynamicMaterialInstance` (`self.SM_Parent`) 0 "/Game/Puzzle3/Lasers/M_TargetHit.M_TargetHit" "None"))
  (`MaterialInstanceDynamic.SetVectorParameterValue` _returnvalue "Base Color" (`KismetMathLibrary.SelectColor` `Color Laser` (struct :`R` 1.0 :`G` 0.01736 :`A` 1.0) (`self.Active`))))

(fn `UserConstructionScript`
  (`parent.UserConstructionScript`))