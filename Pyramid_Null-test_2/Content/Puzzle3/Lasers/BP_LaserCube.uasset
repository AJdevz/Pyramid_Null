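; BP_LaserCube is a puzzle cube that relays an incoming laser out along its arrow's direction.
; LaserBounce switches it active on the first hit, spawning a same-colored BP_Laser with an updated ID, attached to SMParent.
; The new laser is tracked in LasersAttached and the SpawnReference's ChildLasers.
; A negative hit response deactivates the cube and clears all attached lasers.
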(fn `LaserBounce`
  (params (`P-LaserHit` :type "/Game/Puzzle3/Lasers/BP_Laser Object Reference") (`P-HitResponse` :type Boolean) (`P-HitInformation` :type "HitResult Structure"))
  (returns (`New Laser` :type "/Game/Puzzle3/Lasers/BP_Laser Object Reference"))
  (`/Engine/EditorBlueprintResources/StandardMacros.IsValid` `P-LaserHit`
    (:`Is Valid`
      (set `/Game/Puzzle3/Lasers/BP_LasersParent.SpawnReference` null (`/Game/Puzzle3/Lasers/BP_LasersParent.SpawnReference` `P-LaserHit`))
      (if (or (and (`local.P-HitResponse`) (not (`self.Active`))) (not (`local.P-HitResponse`)))
        (bind _output_get (set `self.Active` (`local.P-HitResponse`)))
        (if _output_get
          (bind _returnvalue (`|SpawnActorFromClass` "/Game/Puzzle3/Lasers/BP_Laser.BP_Laser_C" (`KismetMathLibrary.MakeTransform` (`SceneComponent.K2_GetComponentLocation` (`self.Arrow`)) (`KismetMathLibrary.MakeRotFromZ` (`SceneComponent.GetForwardVector` (`self.Arrow`)))) "Undefined" "MultiplyWithRoot" null (`/Game/Puzzle3/Lasers/BP_Laser.Update ID` (`local.P-LaserHit`) "C") (`/Game/Puzzle3/Lasers/BP_LasersParent.LaserColor` (`local.P-LaserHit`)) (`self.SpawnReference`) null))
          (`self.K2_AttachToComponent` _returnvalue (`self.SM_Parent`) "None" "KeepWorld" "KeepWorld" "KeepRelative" false)
          (`KismetArrayLibrary.Array_Add` (`self.LasersAttached`) _returnvalue)
          (`KismetArrayLibrary.Array_Add` (`/Game/Puzzle3/Lasers/BP_LaserSpawn.Child Lasers` (`self.SpawnReference`)) _returnvalue)
          (return _returnvalue)
          (else
            (`self.Clear All Lasers Attached`)))))))

(fn `UserConstructionScript`
  (`parent.UserConstructionScript`))