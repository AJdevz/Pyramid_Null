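; BP_LaserSpawn is a laser emitter actor in Puzzle3 that spawns a BP_Laser when play begins.
; The laser starts at the Arrow component's location with the actor's rotation.
; It receives the spawner's display name as its laser ID, plus the laser color and a reference back to the spawner.
; The spawner stores the new laser in its ChildLasers array.
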(event `self.ReceiveBeginPlay`
  (set `self.SpawnReference` self)
  (set `self.ID` (`KismetSystemLibrary.GetDisplayName` self))
  (bind _returnvalue (`|SpawnActorFromClass` "/Game/Puzzle3/Lasers/BP_Laser.BP_Laser_C" (`KismetMathLibrary.MakeTransform` (`SceneComponent.K2_GetComponentLocation` (`self.Arrow`)) (`self.K2_GetActorRotation`)) "Undefined" "MultiplyWithRoot" null (`self.ID`) (`self.LaserColor`) (`self.SpawnReference`) null))
  (`KismetArrayLibrary.Array_Add` (`self.Child Lasers`) _returnvalue))

(fn `UserConstructionScript`
  (`parent.UserConstructionScript`))