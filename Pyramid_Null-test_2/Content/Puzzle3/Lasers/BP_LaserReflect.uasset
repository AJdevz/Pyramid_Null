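; Reflective surface for the laser puzzle that bounces incoming lasers by spawning new BP_Laser actors at the impact point.
; LaserBounce passes on color and spawn reference, extends the laser ID, and registers each child locally and with the spawn reference.
; Without a hit, it destroys attached lasers whose IDs contain the incoming ID.
; Rotation comes from CalculatesRotation, though its mirror-by-normal math appears unconnected.
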(fn `Clear Attached Lasers`
  (params (`P-ID_Clear` :type String))
  (bind (_arrayindex _arrayelement) (`/Engine/EditorBlueprintResources/StandardMacros.ReverseForEachLoop` (`self.LasersAttached`))
    (:`LoopBody`
      (`/Engine/EditorBlueprintResources/StandardMacros.IsValid` _arrayelement
        (:`Is Valid`
          (if (`KismetStringLibrary.Contains` (`/Game/Puzzle3/Lasers/BP_Laser.Laser_ID` _arrayelement) (`local.P-ID_Clear`))
            (`self.K2_DestroyActor` _arrayelement)
            (`KismetArrayLibrary.Array_RemoveItem` (`self.LasersAttached`) _arrayelement)))))))

(fn `LaserBounce`
  (params (`P-LaserHit` :type "/Game/Puzzle3/Lasers/BP_Laser Object Reference") (`P-HitResponse` :type Boolean) (`P-HitInformation` :type "HitResult Structure"))
  (returns (`New Laser` :type "/Game/Puzzle3/Lasers/BP_Laser Object Reference"))
  (bind _p_laserhit (`local.P-LaserHit`))
  (bind (_bblockinghit _binitialoverlap _time _distance _location _impactpoint _normal _impactnormal _physmat _hitactor _hitcomponent _hitbonename _bonename _hititem _elementindex _faceindex _tracestart) (`GameplayStatics.BreakHitResult` (`local.P-HitInformation`)))
  (if (`local.P-HitResponse`)
    (bind _returnvalue (`|SpawnActorFromClass` "/Game/Puzzle3/Lasers/BP_Laser.BP_Laser_C" (`KismetMathLibrary.MakeTransform` _impactpoint (`KismetMathLibrary.MakeRotFromZ` (`KismetMathLibrary.MirrorVectorByNormal` (- _impactpoint _tracestart) _impactnormal))) "Undefined" "MultiplyWithRoot" null (`/Game/Puzzle3/Lasers/BP_Laser.Update ID` _p_laserhit "B") (`/Game/Puzzle3/Lasers/BP_LasersParent.LaserColor` _p_laserhit) (`/Game/Puzzle3/Lasers/BP_LasersParent.SpawnReference` _p_laserhit) null))
    (`KismetArrayLibrary.Array_Add` (`self.LasersAttached`) _returnvalue)
    (`KismetArrayLibrary.Array_Add` (`/Game/Puzzle3/Lasers/BP_LaserSpawn.Child Lasers` (`/Game/Puzzle3/Lasers/BP_LasersParent.SpawnReference` (`local.P-LaserHit`))) _returnvalue)
    (return _returnvalue)
    (else
      (`self.Clear Attached Lasers` (`/Game/Puzzle3/Lasers/BP_Laser.Laser_ID` (`local.P-LaserHit`))))))

(fn `UserConstructionScript`
  (`parent.UserConstructionScript`))