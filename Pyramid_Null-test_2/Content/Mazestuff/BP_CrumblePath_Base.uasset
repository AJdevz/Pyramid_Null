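; BP_CrumblePath_Base is a path piece of four cubes that crumbles after a qualifying actor stands in its trigger box.
; Overlap by a BPI_PHM_CrumblePath implementer disables that actor's base rotation and starts a Crumble timer; leaving re-enables rotation and clears the timer.
; Crumble loops random rotation jitter on the cubes, then after WobbleTime stops it and turns on physics, without destroying the actor despite DestoyActor's name.
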(event `Wobble`
  (if (`self.canWobble`) :!label _label
    (`KismetSystemLibrary.Delay` 0.1)
    (`SceneComponent.K2_SetWorldRotation` (`self.Cube`) (`KismetMathLibrary.MakeRotator` (`KismetMathLibrary.RandomFloatInRange` -5.0 5.0) (`KismetMathLibrary.RandomFloatInRange` -4.0 4.0) (`KismetMathLibrary.RandomFloatInRange` -3.0 3.0)) false false)
    (`SceneComponent.K2_SetWorldRotation` (`self.Cube1`) (`KismetMathLibrary.MakeRotator` (`KismetMathLibrary.RandomFloatInRange` -5.0 5.0) (`KismetMathLibrary.RandomFloatInRange` -4.0 4.0) (`KismetMathLibrary.RandomFloatInRange` -3.0 3.0)) false false)
    (`SceneComponent.K2_SetWorldRotation` (`self.Cube2`) (`KismetMathLibrary.MakeRotator` (`KismetMathLibrary.RandomFloatInRange` -5.0 5.0) (`KismetMathLibrary.RandomFloatInRange` -4.0 4.0) (`KismetMathLibrary.RandomFloatInRange` -3.0 3.0)) false false)
    (`SceneComponent.K2_SetWorldRotation` (`self.Cube3`) (`KismetMathLibrary.MakeRotator` (`KismetMathLibrary.RandomFloatInRange` -5.0 5.0) (`KismetMathLibrary.RandomFloatInRange` -4.0 4.0) (`KismetMathLibrary.RandomFloatInRange` -3.0 3.0)) false false)
    (goto _label)))

(event `self.Box.OnComponentBeginOverlap`
  (params (OverlappedComponent :type "PrimitiveComponent Object Reference") (OtherActor :type "Actor Object Reference") (OtherComp :type "PrimitiveComponent Object Reference") (OtherBodyIndex :type Integer) (bFromSweep :type Boolean) (SweepResult :type "HitResult Structure (by ref)"))
  (if (`KismetSystemLibrary.DoesImplementInterface` OtherActor "/Game/Mazestuff/BPI_PHM_CrumblePath.BPI_PHM_CrumblePath_C")
    (message `/Game/Mazestuff/BPI_PHM_CrumblePath.DisableBaseRotation` OtherActor)
    (set `self.canCrumble` true)
    (if (`self.canCrumble`)
      (bind _returnvalue (`KismetSystemLibrary.K2_SetTimer` null "Crumble" (`self.DelaySeconds`))))))

(event `self.Box.OnComponentEndOverlap`
  (params (OverlappedComponent :type "PrimitiveComponent Object Reference") (OtherActor :type "Actor Object Reference") (OtherComp :type "PrimitiveComponent Object Reference") (OtherBodyIndex :type Integer))
  (if (`KismetSystemLibrary.DoesImplementInterface` OtherActor "/Game/Mazestuff/BPI_PHM_CrumblePath.BPI_PHM_CrumblePath_C")
    (message `/Game/Mazestuff/BPI_PHM_CrumblePath.EnableBaseRotation` OtherActor)
    (set `self.canCrumble` true)
    (set `self.canWobble` true)
    (`KismetSystemLibrary.K2_ClearAndInvalidateTimerHandle` (stale `self.Box.OnComponentBeginOverlap` _returnvalue))))

(event `DestoyActor`
  (bind _cube (`self.Cube`))
  (`KismetSystemLibrary.Delay` (`self.WobbleTime`))
  (set `self.canWobble` false)
  (`PrimitiveComponent.SetCollisionEnabled` _cube "QueryAndPhysics")
  (`PrimitiveComponent.SetCollisionEnabled` (`self.Cube1`) "QueryAndPhysics")
  (`PrimitiveComponent.SetCollisionEnabled` (`self.Cube2`) "QueryAndPhysics")
  (`PrimitiveComponent.SetCollisionEnabled` (`self.Cube3`) "QueryAndPhysics")
  (`PrimitiveComponent.SetSimulatePhysics` _cube true)
  (`PrimitiveComponent.SetSimulatePhysics` (`self.Cube1`) true)
  (`PrimitiveComponent.SetSimulatePhysics` (`self.Cube2`) true)
  (`PrimitiveComponent.SetSimulatePhysics` (`self.Cube3`) true))

(fn `Crumble`
  (set `self.canWobble` true)
  (`self.Wobble`)
  (`self.DestoyActor`))

(fn `UserConstructionScript`)