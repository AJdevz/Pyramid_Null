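; Actor that lays out instances on its child Hierarchical Instanced Static Mesh components as a row or a 2D grid.
; The construction script picks the mode from Is2D; row mode steps by GeneralRelativeTransform's location.
; Grid mode uses SetAxis to find two non-zero axes of that offset, falling back to row mode otherwise.
; The grid pass sits inside a RowNumber loop, so it re-adds the same instances each iteration.
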(event `1D HISM Generation`
  (set `self.is2D` false)
  (for _index (range (+ (`self.RowNumber`) 1))
    (set `self.CurrentRelativeTransform` (`KismetMathLibrary.MakeTransform` (* (.location (`self.GeneralRelativeTransform`)) _index)))
    (for _array_element (`SceneComponent.GetChildrenComponents` (`self.DefaultSceneRoot`) false)
      (bind _ashierarchical_instanced_static_mesh_component (cast `HierarchicalInstancedStaticMeshComponent` _array_element))
      (`InstancedStaticMeshComponent.AddInstance` _ashierarchical_instanced_static_mesh_component (`self.CurrentRelativeTransform`) false))))

(event `2D HISM Generation`
  (bind _y (.y (.location (`self.GeneralRelativeTransform`))))
  (set `self.is2D` true)
  (for _index (range (+ (`self.RowNumber`) 1))
    (bind (_transform _x_axis _emptytransform) (`self.SetAxis` (.x (.location (`self.GeneralRelativeTransform`))) _index true "X"))
    (if _emptytransform
      (bind (_transform_2 _x_axis_2 _emptytransform_2) (`self.SetAxis` _y _index true "Y"))
      (if _emptytransform_2
        (`self.1D HISM Generation`)
        (else
          (bind (_transform_3 _x_axis_3 _emptytransform_3) (`self.SetAxis` (.z (.location (`self.GeneralRelativeTransform`))) 0 false "Z" :!label _label))
          (if _emptytransform_3
            (`self.1D HISM Generation`)
            (else
              (for _index_2 (range (+ (`self.RowNumber_X-Axis`) 1)) :!label _label_2
                (for _index_3 (range (+ (`self.RowNumber_Y-Axis`) 1))
                  (set `self.CurrentRelativeTransform` (`KismetMathLibrary.MakeTransform` (+ (* (.location (`self.CurrentRelativeTransform_Y-Axis`)) _index_3) (* (.location (`self.CurrentRelativeTransform_X-Axis`)) _index_2))))
                  (for _array_element (`SceneComponent.GetChildrenComponents` (`self.DefaultSceneRoot`) false)
                    (bind _ashierarchical_instanced_static_mesh_component (cast `HierarchicalInstancedStaticMeshComponent` _array_element))
                    (`InstancedStaticMeshComponent.AddInstance` _ashierarchical_instanced_static_mesh_component (`self.CurrentRelativeTransform`) false))))))))
      (else
        (bind (_transform_4 _x_axis_4 _emptytransform_4) (`self.SetAxis` _y _index false "Y"))
        (if _emptytransform_4
          (goto _label)
          (else
            (goto _label_2)))))))

(fn `SetAxis`
  (params (`Axis Value` :type "Float (double-precision)") (`Row Number Index` :type Integer) (`Set Current Relative Transform X Axis` :type Boolean) (Axis :type String))
  (returns (Transform :type "Transform Structure") (`X Axis` :type Boolean) (EmptyTransform :type Boolean))
  (locals (`Local Location` :type "Vector Structure" :default (0.0 0.0 0.0)))
  (bind _returnvalue (`KismetMathLibrary.MakeTransform` (`local.Local Location`)))
  (switch `string` Axis
    (:`Default`
      (set `local.Local Location` (`KismetMathLibrary.MakeVector` `Axis Value`) :!label _label))
    (:`X`
      (goto _label))
    (:`Y`
      (set `local.Local Location` (`KismetMathLibrary.MakeVector` 0.0 `Axis Value`)))
    (:`Z`
      (set `local.Local Location` (`KismetMathLibrary.MakeVector` 0.0 0.0 `Axis Value`))))
  (if (!= `Axis Value` 0.0)
    (if `Set Current Relative Transform X Axis`
      (bind _output_get (set `self.CurrentRelativeTransform_X-Axis` _returnvalue))
      (return _output_get true false)
      (else
        (bind _output_get_2 (set `self.CurrentRelativeTransform_Y-Axis` _returnvalue))
        (return _output_get_2 false false)))
    (else
      (return (struct) false true))))

(fn `UserConstructionScript`
  (if (`self.is2D`)
    (`self.2D HISM Generation`)
    (else
      (`self.1D HISM Generation`))))